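; BP_FixedCam is a fixed-position camera that becomes the player's view when they enter one of its two trigger volumes.
; The trigger blends the view to this actor and messages the player character with the new camera component; DefaultCamera makes it the starting view.
; View-target events track ActiveCamera, and while active with FocusOnPlayer set, Tick uses RInterpTo to aim the camera at the player.
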(event OnComponentBeginOverlap(StartTriggerA)
  (params (OverlappedComponent :type Primitive%20Component%20Object%20Reference) (OtherActor :type Actor%20Object%20Reference) (OtherComp :type Primitive%20Component%20Object%20Reference) (OtherBodyIndex :type Integer) (bFromSweep :type Boolean) (SweepResult :type Hit%20Result%20Structure%20%28by%20ref%29))
  ;[1 1 1] Set as Active Camera when Trigger is entered by Player
  (bind _yes (Class|BPIPlayer|IsPlayer(Message) OtherActor))
  (if _yes
    (Game|Player|SetViewTargetwithBlend (Game|GetPlayerController 0) self (Variables|Default|GetBlend%20Time) "VTBlend_Linear" 0.0 false)
    (Class|BPIPlayer|UpdateCameraComponent(Message) (Game|GetPlayerCharacter 0) (Variables|Default|GetCamera))))

(event OnComponentBeginOverlap(StartTriggerB)
  (params (OverlappedComponent :type Primitive%20Component%20Object%20Reference) (OtherActor :type Actor%20Object%20Reference) (OtherComp :type Primitive%20Component%20Object%20Reference) (OtherBodyIndex :type Integer) (bFromSweep :type Boolean) (SweepResult :type Hit%20Result%20Structure%20%28by%20ref%29))
  ;[1 1 1] Set as Active Camera when Trigger is entered by Player
  (bind _yes (Class|BPIPlayer|IsPlayer(Message) (stale OnComponentBeginOverlap(StartTriggerA) OtherActor)))
  (if _yes
    (Game|Player|SetViewTargetwithBlend (Game|GetPlayerController 0) self (Variables|Default|GetBlend%20Time) "VTBlend_Linear" 0.0 false)
    (Class|BPIPlayer|UpdateCameraComponent(Message) (Game|GetPlayerCharacter 0) (Variables|Default|GetCamera))))

(event EventBeginPlay
  ;[1 1 1] First Camera Setup
  (if (Variables|Default|GetDefault%20Camera)
    (Game|Player|SetViewTargetwithBlend (Game|GetPlayerController 0) self 0.0 "VTBlend_Linear" 0.0 false)
    ;[1 1 1] Set as Active Camera when Trigger is entered by Player
    (Class|BPIPlayer|UpdateCameraComponent(Message) (Game|GetPlayerCharacter 0) (Variables|Default|GetCamera))))

(event EventTick
  (params (DeltaSeconds :type Float%20%28single-precision%29))
  (bind _camera (Variables|Default|GetCamera))
  ;[1 1 1] LookAtPlayerLogic
  (if (and (Variables|Default|GetActiveCamera) (Variables|Default|GetFocusOnPlayer))
    (Transformation|SetWorldRotation _camera (Math|Interpolation|RInterpTo (Transformation|GetWorldRotation _camera) (Math|Rotator|FindLookatRotation (Transformation|GetWorldLocation (Variables|Default|GetCamera)) (Transformation|GetActorLocation (Game|GetPlayerCharacter 0))) (Utilities|Time|GetWorldDeltaSeconds) 0.0) false false)))

(event EventOnBecomeViewTarget
  (params (PC :type Player%20Controller%20Object%20Reference))
  ;[1 1 1] Current Camera Checks
  (Variables|Default|SetActiveCamera true))

(event EventOnEndViewTarget
  (params (PC :type Player%20Controller%20Object%20Reference))
  ;[1 1 1] Current Camera Checks
  (Variables|Default|SetActiveCamera false))

(fn ConstructionScript)