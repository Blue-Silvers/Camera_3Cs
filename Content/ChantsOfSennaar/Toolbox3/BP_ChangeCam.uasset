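; BP_ChangeCam is a trigger volume that moves the player to another scene behind a black-screen fade.
; When an actor overlaps its Box and passes the IsPlayerMessage check, it plays the WBP_BlackScreen fade forward.
; After a delay set by the same PlaybackSpeed variable, it starts the reverse fade and teleports that actor to NextScene's location.
; Despite the name, it contains no camera logic.
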(event OnComponentBeginOverlap(Box)
  (params (OverlappedComponent :type Primitive%20Component%20Object%20Reference) (OtherActor :type Actor%20Object%20Reference) (OtherComp :type Primitive%20Component%20Object%20Reference) (OtherBodyIndex :type Integer) (bFromSweep :type Boolean) (SweepResult :type Hit%20Result%20Structure%20%28by%20ref%29))
  (bind _playback_speed (Variables|Default|GetPlayback%20Speed))
  (bind _yes (Class|BPIPlayer|IsPlayer(Message) OtherActor))
  (if _yes
    (bind _aswbp_black_screen (Utilities|Casting|CastToWBP_BlackScreen (Variables|Default|GetUserWidget)))
    (Default|FadeinBlack _aswbp_black_screen "Forward" _playback_speed)
    (Utilities|FlowControl|Delay _playback_speed)
    (Default|FadeinBlack _aswbp_black_screen "Reverse" _playback_speed)
    (Transformation|SetActorLocation OtherActor (Transformation|GetActorLocation (Variables|Default|GetNextScene)) false true)))

(fn ConstructionScript)