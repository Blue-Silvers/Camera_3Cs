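; BP_TPS is a third-person player character with Monster Hunter-named Enhanced Input controls, added as a mapping context on BeginPlay.
; Input drives camera look, control-rotation-relative movement, and a roll that only adds forward movement input.
; ModifiCameraValue applies stored arm length, socket offset and FOV to the spring arm and camera on aim release or camera reset.
; Aim start is an empty stub, and camera lock only sets a flag.
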(event EventBeginPlay
  (CallFunction|StartControls))

(event EventTick
  (params (DeltaSeconds :type Float%20%28single-precision%29)))

(event Custom|StartControls
  (bind _asplayer_controller (Utilities|Casting|CastToPlayerController (Pawn|GetController)))
  (Utilities|IsValid (PlayerController|LocalPlayerSubsystems|GetEnhancedInputLocalPlayerSubsystem _asplayer_controller)
    (:Is%20Valid
      (Input|AddMappingContext (PlayerController|LocalPlayerSubsystems|GetEnhancedInputLocalPlayerSubsystem _asplayer_controller) "/Game/TPS/MonsterHunterInput/IMC_MonsterHunterTPS.IMC_MonsterHunterTPS" 0 "(bIgnoreAllPressedKeysUntilRelease=True,bForceImmediately=False,bNotifyUserSettings=False)"))))

(event Input|EnhancedActionEvents|EnhancedInputActionIA_MH_Camera
  (params (ActionValue :type Vector%202D%20Structure) (ElapsedSeconds :type Float%20%28double-precision%29) (TriggeredSeconds :type Float%20%28double-precision%29) (InputAction :type Input%20Action%20Object%20Reference :default "/Game/TPS/MonsterHunterInput/IA_MH_Camera.IA_MH_Camera"))
  (Pawn|Input|AddControllerYawInput (.x ActionValue))
  (Pawn|Input|AddControllerPitchInput (.y ActionValue)))

(event Input|EnhancedActionEvents|EnhancedInputActionIA_MH_Aim
  (params (ActionValue :type Boolean) (ElapsedSeconds :type Float%20%28double-precision%29) (TriggeredSeconds :type Float%20%28double-precision%29) (InputAction :type Input%20Action%20Object%20Reference :default "/Game/TPS/MonsterHunterInput/IA_MH_Aim.IA_MH_Aim"))
  (:Started
    (CallFunction|Aimingon))
  (:Canceled
    (CallFunction|AimingOff :!label _label))
  (:Completed
    (goto _label)))

(event Input|EnhancedActionEvents|EnhancedInputActionIA_MH_LockCam
  (params (ActionValue :type Boolean) (ElapsedSeconds :type Float%20%28double-precision%29) (TriggeredSeconds :type Float%20%28double-precision%29) (InputAction :type Input%20Action%20Object%20Reference :default "/Game/TPS/MonsterHunterInput/IA_MH_LockCam.IA_MH_LockCam"))
  (Variables|Default|SetLockCam true))

(event Input|EnhancedActionEvents|EnhancedInputActionIA_MH_Move
  (params (ActionValue :type Vector%202D%20Structure) (ElapsedSeconds :type Float%20%28double-precision%29) (TriggeredSeconds :type Float%20%28double-precision%29) (InputAction :type Input%20Action%20Object%20Reference :default "/Game/TPS/MonsterHunterInput/IA_MH_Move.IA_MH_Move"))
  (bind _returnvalue (Pawn|GetControlRotation :!class /Script/Engine.Pawn))
  (Pawn|Input|AddMovementInput (Math|Vector|GetForwardVector (Math|Rotator|MakeRotator 0.0 0.0 (.yaw (Pawn|GetControlRotation :!class /Script/Engine.Pawn)))) (.y ActionValue) false)
  (Pawn|Input|AddMovementInput (Math|Vector|GetRightVector (Math|Rotator|MakeRotator (.roll _returnvalue) 0.0 (.yaw _returnvalue))) (.x ActionValue) false))

(event Input|EnhancedActionEvents|EnhancedInputActionIA_MH_ResetCam
  (params (ActionValue :type Boolean) (ElapsedSeconds :type Float%20%28double-precision%29) (TriggeredSeconds :type Float%20%28double-precision%29) (InputAction :type Input%20Action%20Object%20Reference :default "/Game/TPS/MonsterHunterInput/IA_MH_ResetCam.IA_MH_ResetCam"))
  (CallFunction|ResetCam))

(event Input|EnhancedActionEvents|EnhancedInputActionIA_MH_Roll
  (params (ActionValue :type Boolean) (ElapsedSeconds :type Float%20%28double-precision%29) (TriggeredSeconds :type Float%20%28double-precision%29) (InputAction :type Input%20Action%20Object%20Reference :default "/Game/TPS/MonsterHunterInput/IA_MH_Roll.IA_MH_Roll"))
  (:Started
    (Pawn|Input|AddMovementInput (Transformation|GetActorForwardVector) 5.0 false)))

(fn ConstructionScript)

(fn ModifiCameraValue
  (bind _springarm (Variables|Default|GetSpringArm))
  (Variables|/Script/Engine.SpringArmComponent|SetTargetArmLength _springarm (Variables|Default|GetCameraDistance%20to%20character))
  (Variables|/Script/Engine.SpringArmComponent|SetSocketOffset _springarm (Variables|Default|GetBaseCameraPose))
  (Variables|/Script/Engine.CameraComponent|SetFieldOfView (Variables|Default|GetCamera) (Variables|Default|GetFOV)))

(fn Aimingon)

(fn AimingOff
  (CallFunction|ModifiCameraValue))

(fn ResetCam
  (CallFunction|ModifiCameraValue))