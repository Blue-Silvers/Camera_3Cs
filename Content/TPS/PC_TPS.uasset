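; PC_TPS is a player controller that relays Monster Hunter-style third-person Enhanced Input actions to a BP_TPS pawn reference.
; Movement follows control rotation, roll adds forward movement input, and aim, camera lock and camera reset call or set pawn members.
; BeginPlay and camera input are empty: the pawn cast, mapping-context setup and look logic are disconnected, so this graph never assigns the pawn reference.
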(event Input|EnhancedActionEvents|EnhancedInputActionIA_MH_Camera
  (params (ActionValue :type Vector%202D%20Structure) (ElapsedSeconds :type Float%20%28double-precision%29) (TriggeredSeconds :type Float%20%28double-precision%29) (InputAction :type Input%20Action%20Object%20Reference :default "/Game/TPS/MonsterHunterInput/IA_MH_Camera.IA_MH_Camera")))

(event Input|EnhancedActionEvents|EnhancedInputActionIA_MH_Aim
  (params (ActionValue :type Boolean) (ElapsedSeconds :type Float%20%28double-precision%29) (TriggeredSeconds :type Float%20%28double-precision%29) (InputAction :type Input%20Action%20Object%20Reference :default "/Game/TPS/MonsterHunterInput/IA_MH_Aim.IA_MH_Aim"))
  (bind _bp_player (Variables|Default|GetBP_Player))
  (:Started
    (Default|Aimingon _bp_player))
  (:Canceled
    (Default|AimingOff _bp_player :!label _label))
  (:Completed
    (goto _label)))

(event Input|EnhancedActionEvents|EnhancedInputActionIA_MH_LockCam
  (params (ActionValue :type Boolean) (ElapsedSeconds :type Float%20%28double-precision%29) (TriggeredSeconds :type Float%20%28double-precision%29) (InputAction :type Input%20Action%20Object%20Reference :default "/Game/TPS/MonsterHunterInput/IA_MH_LockCam.IA_MH_LockCam"))
  (Variables|/Game/TPS/BP_TPS.BP_TPS_C|SetLockCam (Variables|Default|GetBP_Player) true))

(event Input|EnhancedActionEvents|EnhancedInputActionIA_MH_Move
  (params (ActionValue :type Vector%202D%20Structure) (ElapsedSeconds :type Float%20%28double-precision%29) (TriggeredSeconds :type Float%20%28double-precision%29) (InputAction :type Input%20Action%20Object%20Reference :default "/Game/TPS/MonsterHunterInput/IA_MH_Move.IA_MH_Move"))
  (bind _bp_player (Variables|Default|GetBP_Player))
  (bind _returnvalue (Pawn|GetControlRotation _bp_player :!class /Script/Engine.Pawn))
  (Pawn|Input|AddMovementInput _bp_player (Math|Vector|GetForwardVector (Math|Rotator|MakeRotator 0.0 0.0 (.yaw (Pawn|GetControlRotation _bp_player :!class /Script/Engine.Pawn)))) (.y ActionValue) false)
  (Pawn|Input|AddMovementInput _bp_player (Math|Vector|GetRightVector (Math|Rotator|MakeRotator (.roll _returnvalue) 0.0 (.yaw _returnvalue))) (.x ActionValue) false))

(event Input|EnhancedActionEvents|EnhancedInputActionIA_MH_ResetCam
  (params (ActionValue :type Boolean) (ElapsedSeconds :type Float%20%28double-precision%29) (TriggeredSeconds :type Float%20%28double-precision%29) (InputAction :type Input%20Action%20Object%20Reference :default "/Game/TPS/MonsterHunterInput/IA_MH_ResetCam.IA_MH_ResetCam"))
  (Default|ResetCam (Variables|Default|GetBP_Player)))

(event Input|EnhancedActionEvents|EnhancedInputActionIA_MH_Roll
  (params (ActionValue :type Boolean) (ElapsedSeconds :type Float%20%28double-precision%29) (TriggeredSeconds :type Float%20%28double-precision%29) (InputAction :type Input%20Action%20Object%20Reference :default "/Game/TPS/MonsterHunterInput/IA_MH_Roll.IA_MH_Roll"))
  (bind _bp_player (Variables|Default|GetBP_Player))
  (:Started
    (Pawn|Input|AddMovementInput _bp_player (Transformation|GetActorForwardVector _bp_player) 5.0 false)))

(event EventBeginPlay
  ;[1 1 1] Initiate cast and input
)

(fn ConstructionScript)